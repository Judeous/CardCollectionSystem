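; Hand_BP is a card hand area that tracks the Card_BP actors overlapping it in a Cards array.
; Sphere overlap adds a card, then either teleports it up by a running Z offset and increments that offset if InHand is set, or decrements the offset otherwise.
; Ending actor overlap removes the card from the array.
; Shuffling is unfinished: it starts false, and its Tick loop over Cards has an empty body.
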(event OnComponentBeginOverlap(Sphere)
  (params (OverlappedComponent :type Primitive%20Component%20Object%20Reference) (OtherActor :type Actor%20Object%20Reference) (OtherComp :type Primitive%20Component%20Object%20Reference) (OtherBodyIndex :type Integer) (bFromSweep :type Boolean) (SweepResult :type Hit%20Result%20Structure%20%28by%20ref%29))
  (bind _ascard_bp (Utilities|Casting|CastToCard_BP OtherActor))
  ;[1 1 1] Add the new Card to the array
  (Utilities|Array|Add (Variables|Default|GetCards) _ascard_bp)
  (if (Variables|/Game/BluePrints/Card_BP.Card_BP_C|GetInHand _ascard_bp)
    ;[1 1 1] Calculate the location for the Card in the Hand, then move it to that location
    (Transformation|Teleport _ascard_bp (Math|Vector|MakeVector (.x (.location (Transformation|GetActorTransform _ascard_bp))) (.y (.location (Transformation|GetActorTransform _ascard_bp))) (+ (.z (.location (Transformation|GetActorTransform _ascard_bp))) (Variables|Default|GetNextCardDisplacement))) (.rotation (Transformation|GetActorTransform _ascard_bp)))
    ;[1 1 1] Increment displacement location for the next Card in the stack
    (Variables|Default|SetNextCardDisplacement (+ (Variables|Default|GetNextCardDisplacement) 1.0))
    (else
      ;[1 1 1] Decrement displacement location for the next Card in the stack
      (Variables|Default|SetNextCardDisplacement (- (Variables|Default|GetNextCardDisplacement) 1.0)))))

(event EventBeginPlay
  ;[1 1 1] Sets Shuffling to be false upon start
  (Variables|Default|SetShuffling false))

(event Collision|EventActorEndOverlap
  (params (OtherActor :type Actor%20Object%20Reference))
  ;[1 1 1] Remove the Card from the array when it leaves the area covered by the Hand
  (bind _ascard_bp (Utilities|Casting|CastToCard_BP OtherActor))
  (Utilities|Array|RemoveItem (Variables|Default|GetCards) _ascard_bp))

(event EventTick
  (params (DeltaSeconds :type Float%20%28single-precision%29))
  (if (Variables|Default|GetShuffling)
    (for _index (range 0 (Utilities|Array|Length (Variables|Default|GetCards)))
      _)))

(fn ConstructionScript)