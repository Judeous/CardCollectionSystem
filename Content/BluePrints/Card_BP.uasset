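; Card_BP is a clickable playing card actor that shows its rank and suit.
; On BeginPlay it writes Rank and Suit into two text render components.
; Clicking its Cube toggles InHand, teleporting the card between a fixed, rotated hand position and its stored TableLocation transform.
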(event OnClicked(Cube)
  (params (TouchedComponent :type Primitive%20Component%20Object%20Reference) (ButtonPressed :type Key%20Structure :default "None"))
  (bind _tablelocation (Variables|Default|GetTableLocation))
  (if (Variables|Default|GetInHand)
    (Variables|Default|SetInHand false)
    (Transformation|Teleport (.location _tablelocation) (.rotation _tablelocation))
    (else
      (Variables|Default|SetInHand true)
      (Transformation|Teleport "-780.000000,0.000000,600.000000" "0.000000,90.000000,20.000000"))))

(event EventBeginPlay
  (Rendering|Components|TextRender|SetText (Variables|Default|GetRankTextRender) (Utilities|Text|ToText(String) (Variables|Default|GetRank)))
  (Rendering|Components|TextRender|SetText (Variables|Default|GetSuitTextRender) (Utilities|Text|ToText(String) (Variables|Default|GetSuit))))

(event Collision|EventActorBeginOverlap
  (params (OtherActor :type Actor%20Object%20Reference)))

(event EventTick
  (params (DeltaSeconds :type Float%20%28single-precision%29)))

(fn ConstructionScript)